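; Projectile launcher Blueprint that spawns and throws explosive projectiles homing on the player character.
; SpawnProjectile creates the configured projectile class at the Scene component's location, owned by the launcher, and caches it both generically and as a BP_ExplosiveProjectile.
; ThrowProjectile launches it along ProjectileDirection at the speed from its movement component, passing the player's mesh as homing target.
; The event graph holds only disabled stubs.
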(event EventBeginPlay
  (|CallParentFunction) ; This node is disabled and will not be called.\nDrag off pins to build functionality.
)

(event Collision|EventActorBeginOverlap
  (params (OtherActor :type Actor%20Object%20Reference))
  (|CallParentFunction OtherActor) ; This node is disabled and will not be called.\nDrag off pins to build functionality.
)

(event EventTick
  (params (DeltaSeconds :type Float%20%28single-precision%29))
  (|CallParentFunction DeltaSeconds) ; This node is disabled and will not be called.\nDrag off pins to build functionality.
)

(fn ConstructionScript
  (|CallParentFunction))

(fn SpawnProjectile
  (bind _returnvalue (Class|BaseProjectile|SpawnProjectile self (Variables|Default|GetProjectileClass) (Transformation|GetWorldLocation (Variables|Default|GetScene)) "0, 0, 0"))
  (bind _output_get (Variables|Default|SetProjectile _returnvalue))
  (bind _asbp_explosive_projectile (Utilities|Casting|CastToBP_ExplosiveProjectile _output_get))
  (Variables|Default|SetExplosiveProjectile _asbp_explosive_projectile))

(fn ThrowProjectile
  (Class|BaseProjectile|ThrowProjectile (Variables|Default|GetProjectile) (Variables|Default|GetProjectileDirection) (Class|FluskiProjectileMovementComponent|GetProjectileSpeed (Variables|/Script/FluskiProjectiles.GrenadeProjectile|GetProjectileMovement (Variables|Default|GetProjectile))) (Variables|/Script/Engine.Character|GetMesh (Game|GetPlayerCharacter 0))))