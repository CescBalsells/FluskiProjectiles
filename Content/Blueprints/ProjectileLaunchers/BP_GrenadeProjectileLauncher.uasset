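; Projectile launcher child Blueprint specialized for grenades, overriding the parent's spawn, update and throw-check functions.
; After the parent spawns a projectile, it caches it as a BP_GrenadeProjectile.
; Each update feeds an absolute sine of the grenade's age into its movement component, so charged speed oscillates.
; The throw check accumulates delta time per call and passes once the timer exceeds half the grenade's detonation time.
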(event EventBeginPlay
  (|CallParentFunction) ; This node is disabled and will not be called.\nDrag off pins to build functionality.
)

(event Collision|EventActorBeginOverlap
  (params (OtherActor :type Actor%20Object%20Reference))
  (|CallParentFunction OtherActor) ; This node is disabled and will not be called.\nDrag off pins to build functionality.
)

(event EventTick
  (params (DeltaSeconds :type Float%20%28single-precision%29))
  (|CallParentFunction DeltaSeconds) ; This node is disabled and will not be called.\nDrag off pins to build functionality.
)

(fn ConstructionScript
  (|CallParentFunction))

(fn SpawnProjectile
  (|CallParentFunction)
  (bind _asbp_grenade_projectile (Utilities|Casting|CastToBP_GrenadeProjectile (Variables|Default|GetProjectile)))
  (Variables|Default|SetGrenadeProjectile _asbp_grenade_projectile))

(fn CanThrowProjectile
  (bind _output_get (Variables|Default|SetThrowProjectileTimer (+ (Utilities|Time|GetWorldDeltaSeconds) (Variables|Default|GetThrowProjectileTimer))))
  (return (> _output_get (/ (Variables|/Script/FluskiProjectiles.GrenadeProjectile|GetTimeToDetonate (Variables|Default|GetGrenadeProjectile)) 2.0))))

(fn UpdateProjectile
  (|CallParentFunction)
  ;[1 1 1] Update the charged speed of the projectile
  (Class|FluskiProjectileMovementComponent|UpdateChargedSpeed (Variables|/Script/FluskiProjectiles.BaseProjectile|GetProjectileMovement (Variables|Default|GetGrenadeProjectile)) (Math|Float|Absolute(Float) (Math|Trig|Sin(Radians) (* (Actor|GetGameTimeSinceCreation (Variables|Default|GetGrenadeProjectile)) 0.5)))))