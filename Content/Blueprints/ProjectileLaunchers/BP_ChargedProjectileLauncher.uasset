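; Projectile launcher child Blueprint that spawns a charged projectile and only allows throwing it when its charge is nearly full.
; It extends the parent's spawn step to cache the projectile as a BP_ChargedProjectile.
; Each projectile update feeds an absolute sine of the projectile's age into its charge value and movement component's charged speed.
; The charge therefore oscillates between empty and full, so the throw window opens periodically.
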(event EventBeginPlay
  (|CallParentFunction) ; This node is disabled and will not be called.\nDrag off pins to build functionality.
)

(event Collision|EventActorBeginOverlap
  (params (OtherActor :type Actor%20Object%20Reference))
  (|CallParentFunction OtherActor) ; This node is disabled and will not be called.\nDrag off pins to build functionality.
)

(event EventTick
  (params (DeltaSeconds :type Float%20%28single-precision%29))
  (|CallParentFunction DeltaSeconds) ; This node is disabled and will not be called.\nDrag off pins to build functionality.
)

(fn ConstructionScript
  (|CallParentFunction))

(fn SpawnProjectile
  (|CallParentFunction)
  (bind _asbp_charged_projectile (Utilities|Casting|CastToBP_ChargedProjectile (Variables|Default|GetProjectile)))
  (Variables|Default|SetChargedProjectile _asbp_charged_projectile))

(fn CanThrowProjectile
  (return (>= (Variables|/Script/FluskiProjectiles.ChargedProjectile|GetChargedValue (Variables|Default|GetChargedProjectile)) 0.95)))

(fn UpdateProjectile
  (bind _chargedprojectile (Variables|Default|GetChargedProjectile))
  (bind _returnvalue (Actor|GetGameTimeSinceCreation _chargedprojectile))
  (bind _returnvalue_2 (* _returnvalue 0.5))
  (bind _returnvalue_3 (Math|Trig|Sin(Radians) _returnvalue_2))
  (bind _returnvalue_4 (Math|Float|Absolute(Float) _returnvalue_3))
  (|CallParentFunction)
  ;[1 1 1] Updates the Charged value of the projectile, that goes from 0 to 1
  (Class|ChargedProjectile|UpdateChargedValue (Variables|Default|GetChargedProjectile) _returnvalue_4)
  ;[0.9959 0.6176 1] Updates the charged speed with the Charged Projectile Value
  (Class|FluskiProjectileMovementComponent|UpdateChargedSpeed (Variables|/Script/FluskiProjectiles.BaseProjectile|GetProjectileMovement (Variables|Default|GetChargedProjectile)) _returnvalue_4))