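; Base launcher actor that repeatedly spawns a projectile with a trajectory gizmo and throws it automatically after a short timed delay.
; Each Tick before the throw, it derives direction by rotating its forward vector around its right axis by the throw angle, then updates the gizmo.
; Once thrown, the gizmo is destroyed; when the projectile becomes invalid, a Timeline delays spawning the next pair.
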(event EventBeginPlay
  (CallFunction|SpawnProjectile))

(event Collision|EventActorBeginOverlap
  (params (OtherActor :type Actor%20Object%20Reference)))

(event EventTick
  (params (DeltaSeconds :type Float%20%28single-precision%29))
  (bind _projectilegizmo (Variables|Default|GetProjectileGizmo))
  (Utilities|IsValid (Variables|Default|GetProjectile)
    (:Is%20Valid
      (if (Class|BaseProjectile|IsThrown (Variables|Default|GetProjectile))
        (Utilities|IsValid _projectilegizmo
          (:Is%20Valid
            (Actor|DestroyActor _projectilegizmo)))
        (else
          (CallFunction|UpdateProjectile)
          (bind _canthrow (CallFunction|CanThrowProjectile))
          (if _canthrow
            (CallFunction|ThrowProjectile)
            (Variables|Default|SetThrowProjectileTimer 0.0)))))
    (:Is%20Not%20Valid
      (Timeline|Timeline Play
        (:Finished
          (CallFunction|SpawnProjectile))))))

(fn ConstructionScript)

(fn UpdateProjectileGizmo
  (bind _projectilegizmo (Variables|Default|GetProjectileGizmo))
  (bind _projectile (Variables|Default|GetProjectile))
  (Utilities|IsValid _projectilegizmo
    (:Is%20Valid
      (Class|BaseProjectileGizmo|UpdateGizmo _projectilegizmo self (Variables|/Script/FluskiProjectiles.GrenadeProjectile|GetProjectileMovement _projectile) (Variables|/Script/Engine.SphereComponent|GetSphereRadius (Variables|/Script/FluskiProjectiles.GrenadeProjectile|GetCollisionComponent _projectile)) (Variables|Default|GetProjectileDirection)))))

(fn UpdateDirection
  (Variables|Default|SetProjectileDirection (Math|Vector|RotateVectorAroundAxis (Transformation|GetActorForwardVector) (Variables|Default|GetThrowProjectileAngle) (Transformation|GetActorRightVector))))

(fn SpawnProjectile
  (bind _returnvalue (Class|BaseProjectile|SpawnProjectile self (Variables|Default|GetProjectileClass) (Transformation|GetWorldLocation (Variables|Default|GetScene)) "0, 0, 0"))
  (Variables|Default|SetProjectile _returnvalue)
  (bind _returnvalue_2 (Game|SpawnActorfromClass "/FluskiProjectiles/Blueprints/ProjectileGizmos/BP_BaseProjectileGizmo.BP_BaseProjectileGizmo_C" (Math|Transform|MakeTransform (Transformation|GetWorldLocation (Variables|Default|GetScene))) "AdjustIfPossibleButAlwaysSpawn" self 0))
  (Variables|Default|SetProjectileGizmo _returnvalue_2))

(fn ThrowProjectile
  (Class|BaseProjectile|ThrowProjectile (Variables|Default|GetProjectile) (Variables|Default|GetProjectileDirection) (Class|FluskiProjectileMovementComponent|GetProjectileSpeed (Variables|/Script/FluskiProjectiles.GrenadeProjectile|GetProjectileMovement (Variables|Default|GetProjectile))) 0))

(fn UpdateProjectile
  (CallFunction|UpdateDirection)
  (CallFunction|UpdateProjectileGizmo))

(fn CanThrowProjectile
  (bind _output_get (Variables|Default|SetThrowProjectileTimer (+ (Utilities|Time|GetWorldDeltaSeconds) (Variables|Default|GetThrowProjectileTimer))))
  (return (> _output_get 2.0)))